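; BP_RespawnPoint is an enemy spawner that creates BP_EnemyBase actors at random points within the bounds of its SpawnArea component.
; BeginPlay or PerformOneTest resets the counter, spawns one enemy immediately, then repeats on a looping two-second timer.
; When the counter reaches NumberOfEnemiesToSpawn, the next tick of that timer fires the AllSpawned dispatcher and clears the timer.
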(event Custom|DoSpawn
  (bind _spawntimerhandle (Variables|Default|GetSpawnTimerHandle))
  (if (== (Variables|Default|GetNumberOfEnemiesToSpawn) (Variables|Default|GetCurrentEnemyCounter))
    (Default|CallAllSpawned)
    (if (Utilities|Time|IsValidTimerHandle _spawntimerhandle)
      (Utilities|Time|ClearandInvalidateTimerbyHandle _spawntimerhandle))
    (else
      (Variables|Default|SetCurrentEnemyCounter (+ (Variables|Default|GetCurrentEnemyCounter) 1))
      (CallFunction|SpawnEnemy))))

(event Custom|PerformOneTest
  (Variables|Default|SetCurrentEnemyCounter 0)
  (CallFunction|DoSpawn)
  (bind _returnvalue (Utilities|Time|SetTimerbyEvent (delegate Custom|DoSpawn) 2.0 true))
  (Variables|Default|SetSpawnTimerHandle _returnvalue))

(event EventBeginPlay
  (Variables|Default|SetCurrentEnemyCounter 0)
  (CallFunction|DoSpawn)
  (bind _returnvalue (Utilities|Time|SetTimerbyEvent (delegate Custom|DoSpawn) 2.0 true))
  (Variables|Default|SetSpawnTimerHandle _returnvalue))

(event EventTick
  (params (DeltaSeconds :type Float%20%28single-precision%29)))

(fn ConstructionScript)

(fn SpawnEnemy
  (bind _spawnarea (Variables|Default|GetSpawnArea))
  (bind (_origin _boxextent) (Collision|GetComponentBounds _spawnarea))
  (Game|SpawnActorfromClass "/Game/Characters/Enemy/BP_EnemyBase.BP_EnemyBase_C" (Math|Conversions|ToTransform(Vector) (Math|Random|RandomPointinBoundingBox _origin _boxextent)) "Undefined" "MultiplyWithRoot" self 0))
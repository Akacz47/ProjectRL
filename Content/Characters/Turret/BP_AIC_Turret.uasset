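; AI controller for turrets that runs the turret's behavior tree and picks an enemy to attack.
; On possess it caches the turret's location and writes its arrow's forward vector to the Blackboard.
; Sight perception updates select the nearest sensed "Enemy"-tagged actor, replacing the current target only if closer or the current one is invalid.
; The target goes to the Blackboard, and a helper exposes the should-shoot flag.
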(event OnPerceptionUpdated(AIPerception)
  (params (UpdatedActors :type Array%20of%20Actor%20Object%20References))
  (bind _attacktarget (Variables|Default|GetAttackTarget))
  (Variables|Default|SetChoosenTarget 0)
  (Variables|Default|SetMinDistance 99999999.0)
  (for _array_element UpdatedActors
    (bind _sensed (CallFunction|SenseActor _array_element "NewEnumerator1"))
    (if _sensed
      (if (and (< (Math|Vector|Distance(Vector) (Variables|Default|GetTurretLocation) (Transformation|GetActorLocation _array_element)) (Variables|Default|GetMinDistance)) (Actor|ActorHasTag _array_element "Enemy"))
        (Variables|Default|SetChoosenTarget _array_element)
        (Variables|Default|SetMinDistance (Math|Vector|Distance(Vector) (Variables|Default|GetTurretLocation) (Transformation|GetActorLocation _array_element))))))
  (Utilities|IsValid _attacktarget
    (:Is%20Valid
      (if (< (Variables|Default|GetMinDistance) (Math|Vector|Distance(Vector) (Variables|Default|GetTurretLocation) (Transformation|GetActorLocation _attacktarget)))
        (CallFunction|HandleSensedSight (Variables|Default|GetChoosenTarget) :!label _label)))
    (:Is%20Not%20Valid
      (goto _label))))

(event EventPossess
  (params (PossessedPawn :type Pawn%20Object%20Reference))
  (bind _asbp_turret (Utilities|Casting|CastToBP_Turret PossessedPawn))
  (bind _behaviourtree (Variables|/Game/Characters/Turret/BP_Turret.BP_Turret_C|GetBehaviourTree _asbp_turret)
    (:then
      (AI|RunBehaviorTree _behaviourtree)
      (CallFunction|SetForwardVector)
      (Variables|Default|SetTurretLocation (Transformation|GetActorLocation (Pawn|GetControlledPawn))))
    (:else)))

(fn ConstructionScript)

(fn SenseActor
  (params (Actor :type Actor%20Object%20Reference) (Sense :type E_AiSense%20Enum :default "NewEnumerator0"))
  (bind _info (Class|AIPerceptionComponent|GetActorsPerception (Variables|Default|GetAIPerception) Actor))
  (for _array_element (.LastSensedStimuli (Utilities|Struct|BreakActorPerceptionBlueprintInfo _info))
    (bind _returnvalue (Class|AIPerceptionSystem|GetSenseClassforStimulus _array_element))
    (if (== _returnvalue (Utilities|Select :Index Sense :NewEnumerator0 0 :NewEnumerator1 "/Script/AIModule.AISense_Sight"))
      (return (.bSuccessfullySensed (Utilities|Struct|BreakAIStimulus _array_element)) _array_element))))

(fn HandleSensedSight
  (params (Actor :type Actor%20Object%20Reference))
  (AI|Components|Blackboard|SetValueasObject (Variables|Default|GetBlackboard) (Variables|Default|GetAttackTargetKeyName) Actor)
  (Variables|Default|SetAttackTarget Actor))

(fn SetShouldShoot
  (params (ShouldShoot :type Boolean))
  (AI|Components|Blackboard|SetValueasBool (Variables|Default|GetBlackboard) (Variables|Default|GetShouldShootKeyName) ShouldShoot))

(fn SetForwardVector
  (bind _asbp_turret (Utilities|Casting|CastToBP_Turret (Pawn|GetControlledPawn)))
  (AI|Components|Blackboard|SetValueasVector (Variables|Default|GetBlackboard) (Variables|Default|GetForwardVectorKeyName) (Math|Vector|GetForwardVector (Variables|/Game/Characters/Turret/BP_Turret.BP_Turret_C|GetArrow _asbp_turret))))